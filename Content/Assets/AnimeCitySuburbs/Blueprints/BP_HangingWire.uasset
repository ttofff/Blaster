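; BP_HangingWire is a placeable wire point that hangs a cable to the next linked point, for chaining overhead wires.
; The construction script sets Cable01's end to the NextWirePoint's Sphere01 position, converted into local space.
; Sag comes from cable gravity scale, either randomized on each construction run or taken from HangValue.
; Without a valid next point the cable is destroyed; the ResetWires branch and event graph do nothing.
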(fn `UserConstructionScript`
  (if (`self.ResetWires`)
    _
    (else
      _))
  (`/Engine/EditorBlueprintResources/StandardMacros.IsValid` (`self.NextWirePoint`)
    (:`Is Valid`
      (set `CableComponent.EndLocation` (`KismetMathLibrary.InverseTransformLocation` (`self.GetTransform`) (`SceneComponent.K2_GetComponentLocation` (`/Game/Assets/AnimeCitySuburbs/Blueprints/BP_HangingWire.Sphere01` (`self.NextWirePoint`)))) (`self.Cable01`))
      (if (`self.RandomHangingValue`)
        (set `CableComponent.CableGravityScale` (`KismetMathLibrary.RandomFloatInRange` 1.0 10.0) (`self.Cable01`))
        (else
          (set `CableComponent.CableGravityScale` (`self.HangValue`) (`self.Cable01`)))))
    (:`Is Not Valid`
      (`ActorComponent.K2_DestroyComponent` (`self.Cable01`)))))