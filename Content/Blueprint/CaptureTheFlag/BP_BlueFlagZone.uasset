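; Blue flag zone actor for Capture the Flag, with its visible setup done entirely in the Construction Script.
; It tints the zone particle effect with blue-violet colors and scales the effect's height and radius from the ZoneSphere radius.
; When a Flag is assigned, it moves that flag to the zone's X/Y position while keeping the flag's own height.
; The event graph holds no active logic.
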(event `self.ReceiveBeginPlay`)

(fn `UserConstructionScript`
  (bind (_returnvalue_x _returnvalue_y) (`KismetMathLibrary.BreakVector` (`self.K2_GetActorLocation`)))
  (bind _flag (`self.Flag`))
  (bind _zonparticlecomponent (`self.ZonParticleComponent`))
  (bind (_returnvalue_x_2 _returnvalue_y_2 _returnvalue_z) (`KismetMathLibrary.BreakVector` (`self.K2_GetActorLocation` _flag)))
  (bind _returnvalue (/ (`SphereComponent.SphereRadius` (`self.ZoneSphere`)) 60.0))
  (`FXSystemComponent.SetColorParameter` _zonparticlecomponent "Color_1" (struct :`R` 1.508173 :`G` 0.100001 :`B` 10.0 :`A` 1.0))
  (`FXSystemComponent.SetColorParameter` _zonparticlecomponent "Color_2" (struct :`G` 1.15 :`B` 5.0 :`A` 1.0))
  (`NiagaraComponent.SetVariableFloat` _zonparticlecomponent "Height" _returnvalue)
  (`NiagaraComponent.SetVariableFloat` _zonparticlecomponent "Radius" _returnvalue)
  (`/Engine/EditorBlueprintResources/StandardMacros.IsValid` _flag
    (:`Is Valid`
      (`self.K2_SetActorLocation` _flag (`KismetMathLibrary.MakeVector` _returnvalue_x _returnvalue_y _returnvalue_z) false false))))